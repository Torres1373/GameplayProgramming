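; Enemy actor that carries a gun but has no shooting logic, taking damage until it dies.
; On BeginPlay it snaps the gun to a mesh socket and increments the EnemiesLeft count in FirstPersonGameMode.
; Incoming damage lowers clamped Health and plays a hit sound.
; At zero Health it plays a death sound, decrements that count and destroys itself.
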(event `self.ReceiveAnyDamage`
  (params (Damage :type "Float (single-precision)") (DamageType :type "DamageType Object Reference") (InstigatedBy :type "Controller Object Reference") (DamageCauser :type "Actor Object Reference"))
  (bind _returnvalue (`self.K2_GetActorLocation`))
  ;[1 0 0] Take Damage
  (bind _output_get (set `self.Health` (`KismetMathLibrary.FClamp` (- (`self.Health`) Damage) 0.0 100.0)))
  (if (== _output_get 0.0)
    (`GameplayStatics.PlaySoundAtLocation` "/Game/SFX/Death/DeathCUe.DeathCue" _returnvalue (struct) 1.0 1.0 0.0 null null null)
    ;[1 0.0317 0.8354] Decrease number of enemies alive
    (bind _asfirst_person_game_mode (cast `/Game/FirstPersonBP/Blueprints/FirstPersonGameMode` (`GameplayStatics.GetGameMode`)))
    (set `/Game/FirstPersonBP/Blueprints/FirstPersonGameMode.EnemiesLeft` (- (`/Game/FirstPersonBP/Blueprints/FirstPersonGameMode.EnemiesLeft` _asfirst_person_game_mode) 1) _asfirst_person_game_mode)
    (`self.K2_DestroyActor`)
    (else
      (`GameplayStatics.PlaySoundAtLocation` "/Game/SFX/Damage/DamageCue.DamageCue" _returnvalue (struct) 1.0 1.0 0.0 null null null))))

(event `self.ReceiveBeginPlay`
  ;[1 1 1] Gun
  (`|ExecutionSequence`
    (:`then_0`
      (`SceneComponent.K2_AttachToComponent` (`self.Gun`) (`self.Mesh`) "gunSocket" "SnapToTarget" "SnapToTarget" "SnapToTarget" true))
    (:`then_1`
      ;[0.01923 0.02986 1] Add enemy to the count
      (bind _asfirst_person_game_mode (cast `/Game/FirstPersonBP/Blueprints/FirstPersonGameMode` (`GameplayStatics.GetGameMode`)))
      (set `/Game/FirstPersonBP/Blueprints/FirstPersonGameMode.EnemiesLeft` (+ (`/Game/FirstPersonBP/Blueprints/FirstPersonGameMode.EnemiesLeft` _asfirst_person_game_mode) 1) _asfirst_person_game_mode))))

(fn `UserConstructionScript`)